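; Enemy pawn that reloads or opens ThirdPersonMap when its Box collision overlaps BP_Player.
; RandomRoam sends it via AIMoveTo to a random reachable nearby point, but runs once per call and is not called in this Blueprint.
; A looping chase of the player character is present but disconnected, and BeginPlay is empty, so nothing here starts movement.
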(event `RandomRoam`
  (`|AIMoveTo` self (`NavigationSystemV1.K2_GetRandomReachablePointInRadius` (`self.K2_GetActorLocation`) 2000.0 null null) null
    (:`then`
      (`KismetSystemLibrary.Delay` (`KismetMathLibrary.RandomFloatInRange` 0.0)))))

(event `self.ReceiveBeginPlay`)

(event `self.Box.OnComponentBeginOverlap`
  (params (OverlappedComponent :type "PrimitiveComponent Object Reference") (OtherActor :type "Actor Object Reference") (OtherComp :type "PrimitiveComponent Object Reference") (OtherBodyIndex :type Integer) (bFromSweep :type Boolean) (SweepResult :type "HitResult Structure (by ref)"))
  (cast `/Game/BluePrints/Characters/BP_Player` OtherActor)
  (`GameplayStatics.OpenLevelBySoftObjectPtr` "/Game/ThirdPerson/Maps/ThirdPersonMap.ThirdPersonMap"))

(fn `UserConstructionScript`)