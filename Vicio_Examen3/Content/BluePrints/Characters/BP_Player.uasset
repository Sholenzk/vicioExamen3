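; BP_Player is a cursor-aimed player character that moves and fires projectiles and missiles.
; BeginPlay adds the Enhanced Input context, shows the cursor and applies downward pitch input; Tick yaws the actor toward the cursor's hit point.
; Movement follows the actor's own forward and right vectors, so it is relative to the aim.
; Left and right mouse spawn BP_Projectile and BP_Misil at ShootingPoint, with the missile's ammo logic left unconnected.
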(event `self.ReceiveBeginPlay`
  (bind _returnvalue (`GameplayStatics.GetPlayerController` 0))
  ;[0.8508 1 0.187] Mapping context
  (`|ExecutionSequence`
    (:`then_0`
      (`EnhancedInputSubsystemInterface.AddMappingContext` (pcsubsystem `EnhancedInputLocalPlayerSubsystem` _returnvalue) "/Game/BluePrints/Input/IMC_Player.IMC_Player" 0 (struct)))
    (:`then_1`
      ;[0.6709 1 0.522] Mouse View Rotation
      (set `PlayerController.bShowMouseCursor` true _returnvalue))
    (:`then_2`
      (`self.AddControllerPitchInput` -90.0))))

(event `self.ReceiveTick`
  (params (DeltaSeconds :type "Float (single-precision)"))
  (bind (_returnvalue_roll _returnvalue_pitch _returnvalue_yaw) (`KismetMathLibrary.BreakRotator` (`KismetMathLibrary.FindLookAtRotation` (`self.K2_GetActorLocation`) (`.ImpactPoint` (`GameplayStatics.BreakHitResult` (`PlayerController.GetHitResultUnderCursorByChannel` (`GameplayStatics.GetPlayerController` 0) "TraceTypeQuery1" true))))))
  ;[0.6709 1 0.522] Mouse View Rotation
  (`self.K2_SetActorRotation` (`KismetMathLibrary.MakeRotator` 0.0 0.0 _returnvalue_yaw)))

(event `EnhancedInput|/Game/BluePrints/Input/IA_Player`
  (params (ActionValue :type "Vector2D Structure") (ElapsedSeconds :type "Float (double-precision)") (TriggeredSeconds :type "Float (double-precision)") (InputAction :type "InputAction Object Reference" :default "/Game/BluePrints/Input/IA_Player.IA_Player"))
  ;[0.4222 0.2686 1] Movement
  (:`Triggered`
    (`self.AddMovementInput` (* ActionValue_X (`self.GetActorForwardVector`)))
    (`self.AddMovementInput` (* ActionValue_Y (`self.GetActorRightVector`)))))

(event `EnhancedInput|/Game/BluePrints/Input/IA_Player`
  (params (ActionValue :type "Vector2D Structure") (ElapsedSeconds :type "Float (double-precision)") (TriggeredSeconds :type "Float (double-precision)") (InputAction :type "InputAction Object Reference" :default "/Game/BluePrints/Input/IA_Player.IA_Player")))

(event `EnhancedInput|/Game/BluePrints/Input/IA_LeftMouse`
  (params (ActionValue :type "Float (double-precision)") (ElapsedSeconds :type "Float (double-precision)") (TriggeredSeconds :type "Float (double-precision)") (InputAction :type "InputAction Object Reference" :default "/Game/BluePrints/Input/IA_LeftMouse.IA_LeftMouse"))
  ;[0.2708 0.8821 1] Mouse
  (:`Started`
    (`|SpawnActorFromClass` "/Game/BluePrints/Characters/BP_Projectile.BP_Projectile_C" (`SceneComponent.K2_GetComponentToWorld` (`self.ShootingPoint`)) "AdjustIfPossibleButAlwaysSpawn" "MultiplyWithRoot" null null)))

(event `EnhancedInput|/Game/BluePrints/Input/IA_RighMouse`
  (params (ActionValue :type "Float (double-precision)") (ElapsedSeconds :type "Float (double-precision)") (TriggeredSeconds :type "Float (double-precision)") (InputAction :type "InputAction Object Reference" :default "/Game/BluePrints/Input/IA_RighMouse.IA_RighMouse"))
  ;[0.2708 0.8821 1] Mouse
  (:`Started`
    (if true
      (`|SpawnActorFromClass` "/Game/BluePrints/Characters/BP_Misil.BP_Misil_C" (`SceneComponent.K2_GetComponentToWorld` (`self.ShootingPoint`)) "AdjustIfPossibleButAlwaysSpawn" "MultiplyWithRoot" null null))))

(fn `UserConstructionScript`)